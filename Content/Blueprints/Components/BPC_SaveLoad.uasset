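; BPC_SaveLoad is a component that saves and restores the player's last known transform through a GS_PlayerProgress save in the default slot.
; On BeginPlay it loads an existing save and teleports the player character there, or creates a new save object.
; It then starts an autosave loop that writes the pawn's transform, with a short delay between saves.
; A widget macro wraps loads and saves with loading screens and input-mode switches.
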(event Custom|FindGameSave
  (bind _returnvalue (SaveGame|DoesSaveGameExist (Variables|GameData|Instance|GetDefaultSlot)))
  (if _returnvalue
    (CallFunction|LoadGameSave)
    (else
      (CallFunction|CreateGameSave))))

(event Custom|CreateGameSave
  (bind _returnvalue (SaveGame|CreateSaveGameObject "/Nairobi/Blueprints/PlayerData/GS_PlayerProgress.GS_PlayerProgress_C"))
  (Variables|GameData|Instance|SetActiveGame _returnvalue))

(event Custom|LoadGameSave
  (Utilities|LoadUnloadWidget "/Nairobi/Blueprints/UI/LoadingScreen.LoadingScreen_C" :!label _label
    (:Loaded
      (bind _returnvalue (SaveGame|LoadGamefromSlot (Variables|GameData|Instance|GetDefaultSlot)))
      (Utilities|IsValid _returnvalue
        (:Is%20Valid
          (Variables|GameData|Instance|SetActiveGame (.AsGS%20Player%20Progress (Utilities|Casting|CastToGS_PlayerProgress _returnvalue)))
          (goto _label Unload))))
    (:Unloaded
      (Utilities|SaveLocalVariables)
      (Utilities|UpdatePlayerDetails))))

(event Custom|Save%20Game
  (Utilities|SaveGameVariables :!label _label)
  (Utilities|FlowControl|Delay 0.2)
  (goto _label))

(event EventBeginPlay
  (CallFunction|FindGameSave)
  (CallFunction|SaveGame))

(event EventTick
  (params (DeltaSeconds :type Float%20%28single-precision%29)))