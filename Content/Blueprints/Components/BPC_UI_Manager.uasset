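; UI manager component that creates the player HUD and toggles the phone and main menu.
; On BeginPlay it creates a HUD if none exists, or trims multiple copies to one.
; Enhanced Input toggles the phone through a FlipFlop and the menu by checking for existing widgets.
; Show/hide functions create or remove widgets and switch input mode and cursor, with the main menu also pausing the game.
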(event Custom|CreateHUD
  (bind _foundwidgets (Widget|GetAllWidgetsOfClass "/Nairobi/Blueprints/UI/WBP_PlayerHUD.WBP_PlayerHUD_C" false))
  (if (> (Utilities|Array|Length _foundwidgets) 0)
    (if (> (Utilities|Array|Length _foundwidgets) 1)
      (for (_array_element _array_index) _foundwidgets
        (if (> _array_index 0)
          (Widget|RemovefromParent _array_element)
          (else
            (bind _output_get (Variables|Default|SetPlayerHUD _array_element))
            (Widget|RemovefromParent _output_get)
            (UserInterface|Viewport|AddtoViewport _output_get 0)))))
    (else
      (bind _returnvalue (UserInterface|CreateWidget "/Nairobi/Blueprints/UI/WBP_PlayerHUD.WBP_PlayerHUD_C" (Game|GetPlayerController 0)))
      (bind _output_get_2 (Variables|Default|SetPlayerHUD _returnvalue))
      (UserInterface|Viewport|AddtoPlayerScreen _output_get_2))))

(event Input|EnhancedActionEvents|EnhancedInputActionIA_Phone
  (params (ActionValue :type Boolean) (ElapsedSeconds :type Float%20%28double-precision%29) (TriggeredSeconds :type Float%20%28double-precision%29) (InputAction :type Input%20Action%20Object%20Reference :default "/Nairobi/Blueprints/Input/IA_Phone.IA_Phone"))
  (:Started
    (Utilities|FlowControl|FlipFlop
      (:A
        (Utilities|ShowPhone))
      (:B
        (Utilities|HidePhone)))))

(event Input|EnhancedActionEvents|EnhancedInputActionIA_Menu
  (params (ActionValue :type Boolean) (ElapsedSeconds :type Float%20%28double-precision%29) (TriggeredSeconds :type Float%20%28double-precision%29) (InputAction :type Input%20Action%20Object%20Reference :default "/Nairobi/Blueprints/Input/IA_Menu.IA_Menu"))
  (:Started
    (bind _foundwidgets (Widget|GetAllWidgetsOfClass "/Nairobi/Blueprints/UI/WBP_MainMenu.WBP_MainMenu_C" false))
    (if (Utilities|Array|IsEmpty _foundwidgets)
      (Utilities|ShowMainMenu)
      (else
        (Utilities|HideMainMenu)))))

(event EventBeginPlay
  (CallFunction|CreateHUD))

(event EventTick
  (params (DeltaSeconds :type Float%20%28single-precision%29)))