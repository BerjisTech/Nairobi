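; Vehicle interaction component that gives the player's wheeled vehicle a speed boost.
; BeginPlay adds the vehicle input mapping context to player 0, and the boost action prints a debug string and calls the boost event.
; If player 0's pawn is a WheeledVehiclePawn, each trigger adds a fixed velocity along world X to its mesh physics, regardless of facing.
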(event Custom|Boost%20Vehicle%20Speed
  (bind _returnvalue (Game|Player|GetPlayerPawn 0))
  (bind _aswheeled_vehicle_pawn (Utilities|Casting|CastToWheeledVehiclePawn _returnvalue))
  (bind _mesh (Variables|/Script/ChaosVehicles.WheeledVehiclePawn|GetMesh _aswheeled_vehicle_pawn))
  (if (Class|GameplayStatics|ObjectIsA _returnvalue "/Script/ChaosVehicles.WheeledVehiclePawn")
    (bind _returnvalue_2 (Physics|GetPhysicsLinearVelocity _mesh "None"))
    (Physics|SetPhysicsLinearVelocity _mesh (+ _returnvalue_2 "100.000000,0.000000,0.000000") false "None")))

(event Input|EnhancedActionEvents|EnhancedInputActionIA_Speed_Boost
  (params (ActionValue :type Boolean) (ElapsedSeconds :type Float%20%28double-precision%29) (TriggeredSeconds :type Float%20%28double-precision%29) (InputAction :type Input%20Action%20Object%20Reference :default "/Nairobi/Blueprints/Input/IA_Speed_Boost.IA_Speed_Boost"))
  (:Triggered
    (Development|PrintString "Boosting")
    (CallFunction|BoostVehicleSpeed)))

(event EventBeginPlay
  (Input|AddMappingContext (PlayerController|LocalPlayerSubsystems|GetEnhancedInputLocalPlayerSubsystem (Game|GetPlayerController 0)) "/Nairobi/Blueprints/Input/IMC_Vehcile.IMC_Vehcile" 0 "(bIgnoreAllPressedKeysUntilRelease=True,bForceImmediately=False)"))

(event EventTick
  (params (DeltaSeconds :type Float%20%28single-precision%29)))