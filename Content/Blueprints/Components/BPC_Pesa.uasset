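; BPC_Pesa is a player money component tracking pocket cash, M-Pesa and personal, business and Mbogi bank balances.
; On BeginPlay it finds sibling UI manager and save/load components, loads the balances and shows pocket and M-Pesa amounts on the HUD.
; RewardPlayer adds cash to the pocket, saves and refreshes the HUD.
; Tick also writes every balance and calls SaveGame each frame.
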(event EventBeginPlay
  (Utilities|SetupPlayerData))

(event EventTick
  (params (DeltaSeconds :type Float%20%28single-precision%29))
  (Utilities|UpdateBalances))

(event EventRewardPlayer
  (params (cashReward :type Float%20%28double-precision%29))
  (Variables|Default|SetPesa%20Pocket (+ cashReward (Variables|Default|GetPesa%20Pocket)))
  (Utilities|UpdateBalances)
  (Default|UpdateMoney (Variables|Default|GetPlayer%20HUD) true false (Variables|Default|GetPesa%20Pocket)))