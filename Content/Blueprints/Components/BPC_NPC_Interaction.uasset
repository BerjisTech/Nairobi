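; NPC component that wanders its owning Character between random debug destinations around the player and marks it with an arrow indicator.
; Each tick runs ground and eight-direction traces, then obstacle avoidance and movement.
; Forward hits set a cross-product detour from obstacle bounds, which steering favors over the destination.
; Drops beyond a safe height switch the mesh to physics simulation, with health logic tied to ground distance.
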(event EventBeginPlay
  (bind _returnvalue (Components|GetOwner))
  (bind (_origin _boxextent _sphereradius) (Collision|GetComponentBounds 0))
  (bind _returnvalue_2 (Game|SpawnActorfromClass "/Nairobi/Blueprints/Actors/ArrowIndicator.ArrowIndicator_C" (Math|Transform|MakeTransform (+ _origin (Math|Vector|MakeVector 0.0 0.0 (+ _sphereradius 1e+02))) "0.000000,0.000000,0.000000" "0.500000,0.500000,0.500000") "AlwaysSpawn" "OverrideRootScale" _returnvalue 0))
  (Transformation|AttachActorToActor _returnvalue_2 _returnvalue "None" "KeepRelative" "KeepRelative" "KeepRelative" true))

(event EventTick
  (params (DeltaSeconds :type Float%20%28single-precision%29))
  (Utilities|ActionSequencer))