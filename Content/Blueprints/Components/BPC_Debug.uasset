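; Debug component that provides input shortcuts for teleporting the player and testing money UI.
; The teleport input action moves the player pawn to a random PlayerStart.
; The M key feeds random balance updates to the HUD through the pawn's BPC_UI_Manager.
; A separate UpdateMoneyBalance graph, uncalled here, briefly shows a WBP_Money widget with fake rich-text amounts, reusing any existing child.
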(event Input|EnhancedActionEvents|EnhancedInputActionIA_Teleport
  (params (ActionValue :type Boolean) (ElapsedSeconds :type Float%20%28double-precision%29) (TriggeredSeconds :type Float%20%28double-precision%29) (InputAction :type Input%20Action%20Object%20Reference :default "/Nairobi/Blueprints/Input/IA_Teleport.IA_Teleport"))
  (:Triggered
    (bind _outactors (Actor|GetAllActorsOfClass "/Script/Engine.PlayerStart"))
    (Transformation|SetActorTransform (Game|Player|GetPlayerPawn 0) (Transformation|GetActorTransform (.OutItem (Utilities|Array|Random _outactors))) false true)))

(event EventBeginPlay)

(event EventTick
  (params (DeltaSeconds :type Float%20%28single-precision%29)))

(event Input|KeyboardEvents|M
  (params (Key :type Key%20Structure))
  (bind _returnvalue (Game|Player|GetPlayerPawn 0))
  (bind _returnvalue_2 (Actor|GetComponentbyClass _returnvalue "/Nairobi/Blueprints/Components/BPC_UI_Manager.BPC_UI_Manager_C"))
  (:Pressed
    (Utilities|IsValid _returnvalue_2
      (:Is%20Valid
        (Default|UpdateMoney (Variables|/Nairobi/Blueprints/Components/BPC_UI_Manager.BPC_UI_Manager_C|GetPlayerHUD _returnvalue_2) (== (Math|Random|RandomInteger 2) 1) (== (Math|Random|RandomInteger 2) 1) (Math|Random|RandomFloatinRange 3e+03 3e+04))))))