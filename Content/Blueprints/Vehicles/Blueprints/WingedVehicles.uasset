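; Winged vehicle Blueprint that extends a parent vehicle class and starts play as not grounded.
; All IA_Look trigger states feed the movement component, with X driving yaw, roll and steering, and Y driving pitch and inverted throttle.
; Each tick shows the current speed on a text render and lengthens the back spring arm as speed rises, pulling the camera away.
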(event Input|EnhancedActionEvents|EnhancedInputActionIA_Look
  (params (ActionValue :type Vector%202D%20Structure) (ElapsedSeconds :type Float%20%28double-precision%29) (TriggeredSeconds :type Float%20%28double-precision%29) (InputAction :type Input%20Action%20Object%20Reference :default "/Nairobi/Blueprints/Input/IA_Look.IA_Look"))
  (bind _vehiclemovementcomponent (Variables|Default|GetVehicleMovementComponent))
  (:Triggered
    (Class|ChaosVehicleMovementComponent|SetYawInput _vehiclemovementcomponent (.x ActionValue) :!label _label)
    (Class|ChaosVehicleMovementComponent|SetPitchInput _vehiclemovementcomponent (.y ActionValue))
    (Class|ChaosVehicleMovementComponent|SetRollInput _vehiclemovementcomponent (.x ActionValue))
    (Class|ChaosVehicleMovementComponent|SetThrottleInput _vehiclemovementcomponent (* (.y ActionValue) -1.0))
    (Class|ChaosVehicleMovementComponent|SetSteeringInput _vehiclemovementcomponent (.x ActionValue)))
  (:Started
    (goto _label))
  (:Ongoing
    (goto _label))
  (:Canceled
    (goto _label))
  (:Completed
    (goto _label)))

(event EventBeginPlay
  (|CallParentFunction)
  (Variables|Default|Setis_grounded false))

(event Collision|EventActorBeginOverlap
  (params (OtherActor :type Actor%20Object%20Reference)))

(event EventTick
  (params (DeltaSeconds :type Float%20%28single-precision%29))
  (bind _speedlimit (CallFunction|GetCurrentCarSpeed))
  (|CallParentFunction DeltaSeconds)
  (Rendering|Components|TextRender|SetText (Variables|Default|GetTextRender) (Utilities|Text|ToText(Float) _speedlimit "HalfToEven"))
  (Variables|/Script/Engine.SpringArmComponent|SetTargetArmLength (Variables|Default|GetBackSpringArm) (Math|Float|MapRangeClamped _speedlimit 0.0 4e+02 1.2e+03 3.6e+03)))

(fn ConstructionScript
  (|CallParentFunction))