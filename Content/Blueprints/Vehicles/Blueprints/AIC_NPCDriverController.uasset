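; AI controller that drives NPC vehicles along AIPaths splines every tick.
; Steers toward a speed-scaled look-ahead point on the nearest spline, applying full throttle below SpeedLimit.
; Above it, seven line traces run; front hits trigger CornerIndex speed caps for sharp/hairpin turns, or distance-mapped braking when the player-pawn cast fails.
; The corner check tests player pawn 0, not the controlled pawn, and clear front traces keep full throttle.
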(event Custom|AI%20Drive
  (bind _roads (CallFunction|GetRoads))
  (bind _steering (CallFunction|GetLane _roads))
  (CallFunction|Steer _steering)
  (Utilities|SpeedLimiter (Variables|Default|GetSpeed%20Limit)
    (:UnderSpeedLimit
      (CallFunction|SetInput 1.0 0.0))
    (:OverSpeedLimit
      (CallFunction|LineTracer)
      (if (Math|Boolean|ORBoolean (Variables|Default|GetFrontLineTraceHitResults?) (Variables|Default|GetLeftFrontOffsetLineTraceHitResults?) (Variables|Default|GetRightFrontOffsetLineTraceHitResults?))
        (bind _corner (Utilities|GetCorner)
          (:IsInCorner
            (switch Utilities|FlowControl|Switch|SwitchonE_TurnIndex (Variables|/Nairobi/Blueprints/Vehicles/Blueprints/CornerIndex.CornerIndex_C|GetTurnIndex (.AsCorner%20Index (Utilities|Casting|CastToCornerIndex _corner)))
              (:NewEnumerator0
                (Utilities|SpeedLimiter 2e+01
                  (:UnderSpeedLimit
                    (CallFunction|SetInput 1.0 0.0))
                  (:OverSpeedLimit
                    (CallFunction|SetInput 0.0 1.0))))
              (:NewEnumerator1
                (Utilities|SpeedLimiter 12.0
                  (:UnderSpeedLimit
                    (CallFunction|SetInput 1.0 0.0))
                  (:OverSpeedLimit
                    (CallFunction|SetInput 0.0 1.0))))))
          (:CastFailed
            (Utilities|CasttoVehicleBase (Variables|Default|GetLeftFrontOffsetLineTraceHitResults)
              (:CastSuccess
                _)
              (:CastFailed
                (Utilities|CasttoVehicleBase (Variables|Default|GetFrontLineTraceHitResults)
                  (:CastSuccess
                    _)
                  (:CastFailed
                    (Utilities|CasttoVehicleBase (Variables|Default|GetRightFrontOffsetLineTraceHitResults)
                      (:CastFailed
                        _))))))
            (CallFunction|SetInput 0.0 (Math|Float|MapRangeClamped (.distance (Utilities|Array|Get(acopy) (Variables|Default|GetFrontLineTraceHitResults))) 0.0 (Variables|Default|GetLineTraceRange) 0.0 1.0))))
        (else
          (CallFunction|SetInput 1.0 0.0))))))

(event EventBeginPlay)

(event EventTick
  (params (DeltaSeconds :type Float%20%28single-precision%29))
  (CallFunction|AIDrive))

(fn ConstructionScript)

(fn GetCurrentCarSpeed
  (return (* (Vehicle|GetForwardSpeed (Variables|Default|GetVehicleMovementComponent)) 0.036)))

(fn GetLane
  (params (Spline :type Array%20of%20AI%20Paths%20Object%20References))
  (bind _returnvalue (Pawn|GetControlledPawn))
  (bind _returnvalue_2 (Transformation|GetActorLocation _returnvalue))
  (Variables|Default|Set_spline (Variables|/Nairobi/Blueprints/Actors/AIPaths.AIPaths_C|GetSpline (.AsAIPaths (Utilities|Casting|CastToAIPaths (.ReturnValue (Actor|FindNearestActor (Transformation|GetActorLocation (Pawn|GetControlledPawn)) Spline))))))
  (bind _speedlimit (CallFunction|GetCurrentCarSpeed))
  (return (Math|Float|MapRangeClamped (.yaw (Math|Rotator|Delta(Rotator) (Math|Rotator|FindLookatRotation _returnvalue_2 (Spline|FindLocationClosesttoWorldLocation (Variables|Default|Get_spline) (+ (* (Math|Vector|Normalize (Class|SplineComponent|FindTangentClosesttoWorldLocation (Variables|Default|Get_spline) (Transformation|GetActorLocation (Pawn|GetControlledPawn)) "World")) (Math|Float|MapRangeClamped _speedlimit 2e+01 8e+01 5e+01 5e+02)) _returnvalue_2) "World")) (Transformation|GetActorRotation (Pawn|GetControlledPawn)))) -9e+01 9e+01 -1.0 1.0)))

(fn GetRoads
  (bind _outactors (Actor|GetAllActorsOfClass "/Nairobi/Blueprints/Actors/AIPaths.AIPaths_C"))
  (return _outactors))

(fn Steer
  (params (Steering :type Float%20%28single-precision%29))
  (Class|ChaosVehicleMovementComponent|SetSteeringInput (Variables|Default|GetVehicleMovementComponent) Steering))

(fn SetInput
  (params (Throttle :type Float%20%28single-precision%29) (Brake :type Float%20%28single-precision%29))
  (bind _vehiclemovementcomponent (Variables|Default|GetVehicleMovementComponent))
  (Class|ChaosVehicleMovementComponent|SetThrottleInput _vehiclemovementcomponent Throttle)
  (Class|ChaosVehicleMovementComponent|SetBrakeInput _vehiclemovementcomponent Brake))

(fn LineTracer
  (bind _frontlinetraceorigin (Variables|Default|GetfrontLineTraceOrigin))
  (bind _returnvalue (Transformation|GetWorldLocation _frontlinetraceorigin))
  (for _index (range 0 6)
    (LocalVariables|SetCurrent%20index _index)
    (bind (_outhits _returnvalue_2) (Class|KismetSystemLibrary|LineTraceMultiforObjects (Utilities|Select :Index (LocalVariables|GetCurrent%20index) :Option%200 _returnvalue :Option%201 _returnvalue :Option%202 (Transformation|GetWorldLocation (Variables|Default|GetLineTraceFrontLeftOffset)) :Option%203 _returnvalue :Option%204 (Transformation|GetWorldLocation (Variables|Default|GetLineTraceFrontRightOffset)) :Option%205 _returnvalue :Option%206 _returnvalue) (+ (Utilities|Select :Index (LocalVariables|GetCurrent%20index) :Option%200 _returnvalue :Option%201 _returnvalue :Option%202 (Transformation|GetWorldLocation (Variables|Default|GetLineTraceFrontLeftOffset)) :Option%203 _returnvalue :Option%204 (Transformation|GetWorldLocation (Variables|Default|GetLineTraceFrontRightOffset)) :Option%205 _returnvalue :Option%206 _returnvalue) (* (Math|Vector|RotateVectorAroundAxis (Math|Vector|GetForwardVector (Variables|Default|GetfrontLineTraceOrigin)) (Utilities|Select :Index (LocalVariables|GetCurrent%20index) :Option%200 -9e+01 :Option%201 -45.0 :Option%202 0.0 :Option%203 0.0 :Option%204 0.0 :Option%205 45.0 :Option%206 9e+01) "0.000000,0.000000,1.000000") (Variables|Default|GetLineTraceRange))) (Utilities|Array|MakeArray "ObjectTypeQuery7" "ObjectTypeQuery5" "ObjectTypeQuery3" "ObjectTypeQuery1") false (Utilities|Array|MakeArray (Pawn|GetControlledPawn)) "None" true))
    (Variables|Default|SetOutHitObjects _outhits)
    (Variables|Default|SetLineTraceHit? _returnvalue_2)
    (switch int (LocalVariables|GetCurrent%20index)
      (:0
        (Variables|Default|SetLeftLineTraceHitResults (Variables|Default|GetOutHitObjects))
        (Variables|Default|SetLeftLineTraceHitResults? (Variables|Default|GetLineTraceHit?)))
      (:1
        (Variables|Default|SetLeftFrontLineTraceHitResults (Variables|Default|GetOutHitObjects))
        (Variables|Default|SetLeftFrontLineTraceHitResults? (Variables|Default|GetLineTraceHit?)))
      (:2
        (Variables|Default|SetLeftFrontOffsetLineTraceHitResults (Variables|Default|GetOutHitObjects))
        (Variables|Default|SetLeftFrontOffsetLineTraceHitResults? (Variables|Default|GetLineTraceHit?)))
      (:3
        (Variables|Default|SetFrontLineTraceHitResults (Variables|Default|GetOutHitObjects))
        (Variables|Default|SetFrontLineTraceHitResults? (Variables|Default|GetLineTraceHit?)))
      (:4
        (Variables|Default|SetRightFrontOffsetLineTraceHitResults (Variables|Default|GetOutHitObjects))
        (Variables|Default|SetRightFrontOffsetLineTraceHitResults? (Variables|Default|GetLineTraceHit?)))
      (:5
        (Variables|Default|SetRightFrontLineTraceHitResults (Variables|Default|GetOutHitObjects)))
      (:6
        (Variables|Default|SetRightLineTraceHitResults (Variables|Default|GetOutHitObjects)))))
  (return))