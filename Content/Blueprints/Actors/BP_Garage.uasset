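; BP_Garage is a garage actor that parks vehicles entering its box and opens the garage UI for them.
; On overlap it teleports the vehicle to VehicleParking; with a BPC_Vehicle_Interaction component, it also flags it in-garage, shows GarageUI with mouse input and moves FrontCamera to the BodyCamera transform.
; End overlap removes every GarageUI, restores game input, activates BackCamera and resets FrontSpringArm from DefaultFrontCamera.
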(event OnComponentEndOverlap(Box)
  (params (OverlappedComponent :type Primitive%20Component%20Object%20Reference) (OtherActor :type Actor%20Object%20Reference) (OtherComp :type Primitive%20Component%20Object%20Reference) (OtherBodyIndex :type Integer))
  (bind _returnvalue (Game|GetPlayerController 0))
  (bind _foundwidgets (Widget|GetAllWidgetsOfClass "/Nairobi/Blueprints/UI/GarageUI.GarageUI_C" true))
  (for _array_element _foundwidgets
    (Widget|RemovefromParent _array_element)
    (Input|SetInputModeGameOnly _returnvalue true)
    (Variables|/Script/Engine.PlayerController|SetbShowMouseCursor _returnvalue false)
    (Components|Activation|Deactivate (Variables|/Nairobi/Blueprints/Vehicles/Blueprints/vehicle_base_pawn.vehicle_base_pawn_C|GetFrontCamera (Variables|/Nairobi/Blueprints/UI/GarageUI.GarageUI_C|GetvehicleInGarage _array_element)))
    (Components|Activation|Activate (Variables|/Nairobi/Blueprints/Vehicles/Blueprints/vehicle_base_pawn.vehicle_base_pawn_C|GetBackCamera (Variables|/Nairobi/Blueprints/UI/GarageUI.GarageUI_C|GetvehicleInGarage _array_element)) false)
    (Transformation|SetRelativeTransform (Variables|/Nairobi/Blueprints/Vehicles/Blueprints/vehicle_base_pawn.vehicle_base_pawn_C|GetFrontSpringArm (Variables|/Nairobi/Blueprints/UI/GarageUI.GarageUI_C|GetvehicleInGarage _array_element)) (Transformation|GetRelativeTransform (Variables|/Nairobi/Blueprints/Vehicles/Blueprints/vehicle_base_pawn.vehicle_base_pawn_C|GetdefaultFrontCamera (Variables|/Nairobi/Blueprints/UI/GarageUI.GarageUI_C|GetvehicleInGarage _array_element))) false false)))

(event OnComponentBeginOverlap(Box)
  (params (OverlappedComponent :type Primitive%20Component%20Object%20Reference) (OtherActor :type Actor%20Object%20Reference) (OtherComp :type Primitive%20Component%20Object%20Reference) (OtherBodyIndex :type Integer) (bFromSweep :type Boolean) (SweepResult :type Hit%20Result%20Structure%20%28by%20ref%29))
  (bind _returnvalue (Actor|GetComponentbyClass OtherActor "/Nairobi/Blueprints/Components/BPC_Vehicle_Interaction.BPC_Vehicle_Interaction_C"))
  (bind _returnvalue_2 (Game|GetPlayerController 0))
  (bind _asvehicle_base_pawn (Utilities|Casting|CastTovehicle_base_pawn OtherActor))
  (bind _frontcamera (Variables|/Nairobi/Blueprints/Vehicles/Blueprints/vehicle_base_pawn.vehicle_base_pawn_C|GetFrontCamera _asvehicle_base_pawn))
  (if (Class|GameplayStatics|ObjectIsA OtherActor "/Nairobi/Blueprints/Vehicles/Blueprints/vehicle_base_pawn.vehicle_base_pawn_C")
    (Transformation|SetActorTransform OtherActor (Transformation|GetWorldTransform (Variables|Default|GetVehicleParking)) false true)
    (Utilities|IsValid _returnvalue
      (:Is%20Valid
        (Variables|/Nairobi/Blueprints/Components/BPC_Vehicle_Interaction.BPC_Vehicle_Interaction_C|Setis_in_garage _returnvalue true)
        (bind _returnvalue_3 (UserInterface|CreateWidget "/Nairobi/Blueprints/UI/GarageUI.GarageUI_C"))
        (UserInterface|Viewport|AddtoViewport _returnvalue_3 0)
        (Input|SetInputModeUIOnly _returnvalue_2 _returnvalue_3 "DoNotLock" false)
        (Variables|/Nairobi/Blueprints/UI/GarageUI.GarageUI_C|SetvehicleInGarage _returnvalue_3 _asvehicle_base_pawn)
        (Variables|/Script/Engine.PlayerController|SetbShowMouseCursor _returnvalue_2 true)
        (Physics|SetPhysicsLinearVelocity (Variables|/Script/ChaosVehicles.WheeledVehiclePawn|GetMesh _asvehicle_base_pawn) "0, 0, 0" true "None")
        (Components|Activation|Deactivate _frontcamera)
        (Components|Activation|Activate _frontcamera false)
        (Transformation|SetRelativeTransform _frontcamera (Transformation|GetRelativeTransform (Variables|/Nairobi/Blueprints/Vehicles/Blueprints/vehicle_base_pawn.vehicle_base_pawn_C|GetbodyCamera _asvehicle_base_pawn)) false true)))))

(event EventBeginPlay)

(event Collision|EventActorBeginOverlap
  (params (OtherActor :type Actor%20Object%20Reference)))

(event EventTick
  (params (DeltaSeconds :type Float%20%28single-precision%29)))

(fn ConstructionScript)