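; BP_Collectible is a spinning pickup actor with a type of Money or Flossin Mauwano.
; On BeginPlay it picks a mesh by type and adds one Instanced Static Mesh instance at the actor's transform, then yaws every tick.
; When a character overlaps the mesh, Money pays CashReward through that actor's BPC_Pesa component and destroys the pickup.
; Flossin Mauwano has a mesh but no overlap behavior.
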(event OnComponentBeginOverlap(InstancedStaticMesh)
  (params (OverlappedComponent :type Primitive%20Component%20Object%20Reference) (OtherActor :type Actor%20Object%20Reference) (OtherComp :type Primitive%20Component%20Object%20Reference) (OtherBodyIndex :type Integer) (bFromSweep :type Boolean) (SweepResult :type Hit%20Result%20Structure%20%28by%20ref%29))
  (bind _returnvalue (Actor|GetComponentbyClass OtherActor "/Nairobi/Blueprints/Components/BPC_Pesa.BPC_Pesa_C"))
  (Utilities|IsCharacter OtherActor
    (:yes
      (switch Utilities|FlowControl|Switch|SwitchonE_CollectibleTypes (Variables|Default|GetcollectibleType)
        (:NewEnumerator0
          (Utilities|IsValid _returnvalue
            (:Is%20Valid
              (Default|RewardPlayer _returnvalue (Variables|Default|GetcashReward))
              (Actor|DestroyActor))))))))

(event EventBeginPlay
  (Utilities|SetUpCollectible))

(event Collision|EventActorBeginOverlap
  (params (OtherActor :type Actor%20Object%20Reference)))

(event EventTick
  (params (DeltaSeconds :type Float%20%28single-precision%29))
  (Transformation|SetActorRotation (Math|Rotator|MakeRotator 0.0 0.0 (+ (.yaw (Transformation|GetActorRotation)) 2.0)) true))

(fn ConstructionScript)