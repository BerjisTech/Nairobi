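; Spline tool actor that tiles a static mesh along a spline as undeformed instances.
; The construction script fills an InstancedStaticMesh component, spacing copies by the mesh's X bounds plus an offset to fit the spline length.
; Each instance is aimed at the next sampled spline point, with configurable location, rotation and scale adjustments, and actor collision is switchable.
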(event EventBeginPlay)

(event Collision|EventActorBeginOverlap
  (params (OtherActor :type Actor%20Object%20Reference)))

(event EventTick
  (params (DeltaSeconds :type Float%20%28single-precision%29)))

(fn ConstructionScript
  (bind _spline_mesh (Variables|ChangeTheSplineSettingsHere|GetSpline%20Mesh))
  (bind _rotation (Variables|ChangetheSplineSettingsHere|Getrotation))
  (bind _returnvalue (StaticMesh|GetBoundingBox _spline_mesh))
  (bind (_min _max) (Utilities|Struct|BreakBox _returnvalue))
  (Components|StaticMesh|SetStaticMesh (Variables|Default|GetInstancedStaticMesh) (Variables|ChangeTheSplineSettingsHere|GetSpline%20Mesh))
  (Collision|SetActorEnableCollision (Variables|ChangeTheSplineSettingsHere|GetCollision?))
  ;[1 1 1] Tile Next Mesh
  (bind _output_get (Variables|Default|SetSpacing (+ (.X (Math|Vector|BreakVector (- _max _min))) (Variables|ChangeTheSplineSettingsHere|GetSpline%20Mesh%20Offset))))
  (bind _output_get_2 (LocalVariables|SetNumber%20Of%20Instances (Math|Float|Floor (/ (Spline|GetSplineLength (Variables|Default|GetSpline)) _output_get))))
  (for _index (range 0 _output_get_2)
    (Components|InstancedStaticMesh|AddInstance (Variables|Default|GetInstancedStaticMesh) (Math|Transform|MakeTransform (+ (Variables|ChangetheSplineSettingsHere|Getlocation) (CallFunction|GetLocationatIndex _index)) (Math|Rotator|MakeRotator (+ (.roll (Math|Rotator|MakeRotfromX (- (CallFunction|GetLocationatIndex (+ _index 1)) (CallFunction|GetLocationatIndex _index)))) (.roll _rotation)) (+ (.pitch (Math|Rotator|MakeRotfromX (- (CallFunction|GetLocationatIndex (+ _index 1)) (CallFunction|GetLocationatIndex _index)))) (.pitch _rotation)) (+ (.yaw (Math|Rotator|MakeRotfromX (- (CallFunction|GetLocationatIndex (+ _index 1)) (CallFunction|GetLocationatIndex _index)))) (.yaw _rotation))) (Variables|ChangetheSplineSettingsHere|Getscale)) false)))

(fn GetLocationatIndex
  (params (A :type Integer))
  (return (Spline|GetLocationatDistanceAlongSpline (Variables|Default|GetSpline) (* A (Variables|Default|GetSpacing)) "Local")))